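; BP_SGKBuildingInterface is the Blueprint interface for build parts in the Survival Game Kit V2 building system.
; It declares calls for previewing, placing, upgrading and deleting parts, plus queries for part type, state, support, grids and build collision.
; It also covers owner management, building options tied to player inventory, and loading extra data from save games.
; The functions are signatures with only default returns, leaving behavior to implementers.
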(fn SGKDeleteBuildPart
  (params (PlayerBuildingComponent :type BP%20Player%20Building%20Component%20Object%20Reference) (ForceDestroy :type Boolean)))

(fn SGKBuildPartType
  (return "NewEnumerator0"))

(fn SGKIsPendingDestroy
  (return false))

(fn SGKSupportCheck
  (params (DestroyOnFail :type Boolean) (DirectSupportOnly :type Boolean))
  (return false false))

(fn SGKIsPlaced
  (return false))

(fn SGKBuildingOptions
  (params (PlayerInventory :type BP%20Player%20Inventory%20Object%20Reference)))

(fn SGKBuildPart
  (return ""))

(fn SGKIsOwner
  (params (PlayerName :type Text))
  (return false))

(fn SGKBuildPartPlaced
  (params (PlayerInventory :type BP%20Player%20Inventory%20Object%20Reference) (FromSaveGame :type Boolean)))

(fn SGKUpgrade)

(fn SGKAddOwner
  (params (PlayerName :type Text))
  (return false))

(fn SGKClearOwners
  (return false))

(fn SGKAddMultipleOwners
  (params (Owners :type Array%20of%20Texts))
  (return false))

(fn SGKPreview
  (params (Preview :type Boolean))
  (return false))

(fn SGKLoadExtraData
  (params (SaveGame :type BP%20SGK%20Save%20Game%20Object%20Reference) (Index :type Integer)))

(fn SGKBPGrids
  (return 0))

(fn SGKBPBuildCollision
  (return 0))